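; Demo actor that asynchronously loads Blueprint and C++ enemy primary data assets side by side on BeginPlay.
; Each path collects its assets in an array and starts a looping timer once all have loaded.
; The Blueprint path async-loads soft skeletal meshes, cycling through the array to display them.
; The C++ path loads the "Visuals" bundle upfront, so hat static meshes resolve directly without another load.
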(event Custom|LoadAllStatic_CPP
  ;[0.15 0 0.05315 0.5] CPP
  (CallFunction|LoadDirectlyCPP))

(event Custom|AllAssetsLoadCPP
  ;[0.15 0 0.05315 0.5] CPP
  (CallFunction|StartTimerLoadCPP))

(event Custom|AllAssetsLoaded
  ;[0 0.02846 0.15 0.5] BP
  (CallFunction|StartTimerLoadBP))

(event Custom|LoadAllSkeletal
  ;[0 0.02846 0.15 0.5] BP
  (|LoadAsyncBP))

(event EventBeginPlay
  (Utilities|FlowControl|Sequence
    (:then_0
      (|ASYNCLOAD_BlueprintPrimaryAsset))
    (:then_1
      (|ASYNCLOAD_CPP))))

(fn ConstructionScript)

(fn StartTimerLoadCPP
  (Development|PrintString "All Primary Assets CPP Loaded")
  (bind _returnvalue (Utilities|Time|SetTimerbyEvent (EventDispatchers|CreateEvent :!event Custom|LoadAllStatic_CPP) 5.0 true))
  (Variables|Default|SetLoadAllMeshHandle_CPP _returnvalue))

(fn LoadDirectlyCPP
  (bind _enmydataarray_cpp (Variables|Default|GetEnmyDataArray_CPP))
  (bind _index_cpp (Variables|Default|GetIndex_CPP))
  (bind _output (Utilities|Array|Get(acopy) _enmydataarray_cpp _index_cpp))
  (bind _hatmesh (Variables|/Script/Unreal2CPP.CPP_EnemyDataAsset|GetHatMesh _output))
  (bind _output_2 (Utilities|ResolveSoftReference _hatmesh))
  (Utilities|IsValid _output_2
    (:Is%20Valid
      (Components|StaticMesh|SetStaticMesh (Variables|Default|GetMESHCPP) _output_2))
    (:Is%20Not%20Valid
      (Development|PrintString "NOT VALID"))))

(fn StartTimerLoadBP
  (Development|PrintString "All Primary Assets Loaded")
  (bind _returnvalue (Utilities|Time|SetTimerbyEvent (EventDispatchers|CreateEvent :!event Custom|LoadAllSkeletal) 2.0 true))
  (Variables|Default|SetLoadAllSkeletalHandle _returnvalue))